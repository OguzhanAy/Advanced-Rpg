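; BP_InsectWeapon is an insect weapon Blueprint that creates Chaos physics fields to fracture and scatter destructible objects.
; Its CreateFields event takes a location and applies external cluster strain through a radial falloff with no attenuation, breaking clusters within the sphere.
; It then applies a filtered linear force from a radial vector centred on that location to push pieces.
; A debug box trace is present but never runs.
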(event `self.CreateFields`
  (params (FieldLocation :type "Vector Structure (by ref)"))
  (bind _fieldsystem (`self.FieldSystem`))
  (`FieldSystemComponent.ApplyPhysicsField` _fieldsystem true "Field_ExternalClusterStrain" null (`RadialFalloff.SetRadialFalloff` (`self.RadialFalloff`) 1000000.0 0.8 1.0 0.0 200.0 FieldLocation "Field_FallOff_None"))
  (`FieldSystemComponent.ApplyPhysicsField` _fieldsystem true "Field_LinearForce" (`self.FieldSystemMetaDataFilter`) (`RadialVector.SetRadialVector` (`self.RadialVector`) 15000000.0 FieldLocation)))

(fn `UserConstructionScript`)