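; Player character Blueprint that adds combat-target lock-on to the Slash character.
; While a CombatTarget is valid, Tick feeds translation and rotation targets to MotionWarping and interpolates controller and actor yaw toward it, the actor with a fixed delta time.
; Without a target, both warp targets are removed.
; Escape quits the game, and mesh overlap with a "Falling"-tagged component prints a debug string and reloads the current level.
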(event `self.ReceiveTick`
  (params (DeltaSeconds :type "Float (single-precision)"))
  (bind _returnvalue (`self.GetController`))
  (bind (_returnvalue_roll _returnvalue_pitch) (`KismetMathLibrary.BreakRotator` (`self.K2_GetActorRotation`)))
  (bind _motionwarping (`self.MotionWarping`))
  (bind _returnvalue_2 (`Controller.GetControlRotation` _returnvalue))
  (`|ExecutionSequence`
    (:`then_0`
      (`self.CombatTarget`
        (:`then`
          (bind _returnvalue_3 (`self.GetTranslationWarpTarget`))
          (`MotionWarpingComponent.AddOrUpdateWarpTargetFromLocation` (`self.MotionWarping`) "TranslationTarget" _returnvalue_3)
          (bind _returnvalue_4 (`self.GetRotationWarpTarget`))
          (`MotionWarpingComponent.AddOrUpdateWarpTargetFromLocation` (`self.MotionWarping`) "RotationTarget" _returnvalue_4))
        (:`else`
          (`MotionWarpingComponent.RemoveWarpTarget` _motionwarping "TranslationTarget")
          (`MotionWarpingComponent.RemoveWarpTarget` _motionwarping "RotationTarget"))))
    (:`then_1`
      (bind _combattarget (`self.CombatTarget`)
        (:`then`
          (`Controller.SetControlRotation` _returnvalue (`KismetMathLibrary.MakeRotator` (.roll _returnvalue_2) (.pitch _returnvalue_2) (.yaw (`KismetMathLibrary.RInterpTo` _returnvalue_2 (`KismetMathLibrary.FindLookAtRotation` (`SceneComponent.K2_GetComponentLocation` (`self.CameraView`)) (`self.K2_GetActorLocation` _combattarget)) (`GameplayStatics.GetWorldDeltaSeconds`) 5.0)))))
        (:`else`)))
    (:`then_2`
      (bind _combattarget_2 (`self.CombatTarget`)
        (:`then`
          (bind (_returnvalue_roll_2 _returnvalue_pitch_2 _returnvalue_yaw) (`KismetMathLibrary.BreakRotator` (`KismetMathLibrary.RInterpTo` (`self.K2_GetActorRotation`) (`KismetMathLibrary.FindLookAtRotation` (`self.K2_GetActorLocation`) (`self.K2_GetActorLocation` _combattarget_2)) 0.4 0.4)))
          (`self.K2_SetActorRotation` (`KismetMathLibrary.MakeRotator` _returnvalue_roll _returnvalue_pitch _returnvalue_yaw)))
        (:`else`)))))

(event `Key|Escape`
  (params (Key :type "Key Structure"))
  (:`Pressed`
    (`KismetSystemLibrary.QuitGame` null "Quit")))

(event `self.Mesh.OnComponentBeginOverlap`
  (params (OverlappedComponent :type "PrimitiveComponent Object Reference") (OtherActor :type "Actor Object Reference") (OtherComp :type "PrimitiveComponent Object Reference") (OtherBodyIndex :type Integer) (bFromSweep :type Boolean) (SweepResult :type "HitResult Structure (by ref)"))
  (if (`ActorComponent.ComponentHasTag` OtherComp "Falling")
    (`KismetSystemLibrary.PrintString` "Hello")
    (bind _returnvalue (`GameplayStatics.GetCurrentLevelName` true))
    (`GameplayStatics.OpenLevel` (`KismetStringLibrary.Conv_StringToName` _returnvalue))))

(fn `UserConstructionScript`)